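; Example actor that drives a BCMultiplay component, loading and playing sets of files through an on-screen WB_Multiplay widget.
; On BeginPlay it shows the cursor, passes debug and base-path settings from BCConfigLoader to the player, then creates the widget.
; Widget events play, stop, or load a folder and extension pair chosen by index.
; The player's finish event calls play again to loop.
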(event OnLoaded(BC_Multiplay)
  (Development|PrintString "loaded files" false))

(event Custom|onButtons
  (params (type :type Integer))
  (switch int type
    (:1
      (Default|PlayAction (Variables|Default|GetBC_Multiplay)))
    (:2
      (Default|StopAction (Variables|Default|GetBC_Multiplay)))))

(event Custom|onCustomClick
  (params (type :type Integer))
  (bind _bc_multiplay (Variables|Default|GetBC_Multiplay))
  (Variables|/MultiPlay/Blueprints/BC_Multiplay.BC_Multiplay_C|Setpath _bc_multiplay (Utilities|Array|Get(acopy) (Variables|Default|Getfolders) type))
  (Variables|/MultiPlay/Blueprints/BC_Multiplay.BC_Multiplay_C|Setextension _bc_multiplay (Utilities|Array|Get(acopy) (Variables|Default|Getextensions) type))
  (Default|LoadAction (Variables|Default|GetBC_Multiplay)))

(event Custom|onFinish
  ;[1 1 1] Loop
  (Default|PlayAction (Variables|Default|GetBC_Multiplay)))

(event EventBeginPlay
  (bind _bc_configloader (Variables|Default|GetBC_ConfigLoader))
  (bind _bc_multiplay (Variables|Default|GetBC_Multiplay))
  (Utilities|FlowControl|Sequence
    (:then_0
      (Variables|/Script/Engine.PlayerController|SetbShowMouseCursor (Game|GetPlayerController 0) true))
    (:then_1
      (Default|LoadAction _bc_configloader)
      (Variables|/MultiPlay/Blueprints/BC_Multiplay.BC_Multiplay_C|SetisDebug _bc_multiplay (Variables|/MultiPlay/Blueprints/BC_ConfigLoader.BC_ConfigLoader_C|GetIs%20Debug _bc_configloader))
      (Variables|/MultiPlay/Blueprints/BC_Multiplay.BC_Multiplay_C|SetbasePath _bc_multiplay (Variables|/MultiPlay/Blueprints/BC_ConfigLoader.BC_ConfigLoader_C|GetBase%20Path _bc_configloader)))
    (:then_2
      ;[1 1 1] Loop
      (EventDispatchers|BindEventtoOnFinish (Variables|Default|GetBC_Multiplay) (delegate Custom|onFinish)))
    (:then_3
      (bind _returnvalue (UserInterface|CreateWidget "/MultiPlay/Blueprints/WB_Multiplay.WB_Multiplay_C" (Game|GetPlayerController 0)))
      (bind _output_get (Variables|Default|Setwidget _returnvalue))
      (UserInterface|Viewport|AddtoViewport _output_get 0)
      (EventDispatchers|BindEventtoButtonEvents _output_get (delegate Custom|onButtons))
      (EventDispatchers|BindEventtoLoadEvents _output_get (delegate Custom|onCustomClick)))))

(event Collision|EventActorBeginOverlap
  (params (OtherActor :type Actor%20Object%20Reference)))

(event EventTick
  (params (DeltaSeconds :type Float%20%28single-precision%29)))

(fn ConstructionScript)

(fn GetDataPath
  (params (file :type String))
  (return (Utilities|String|Append (Class|BlueprintPathsLibrary|ProjectPersistentDownloadDir) "../../../Data/" file)))

(fn GetVideosPath
  (params (file :type String))
  (return (Utilities|String|Append (Class|KismetSystemLibrary|GetProjectDirectory) "Movies/" file)))