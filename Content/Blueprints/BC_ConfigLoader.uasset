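; Config loader Blueprint that reads the game's base path and debug flag from a JSON file.
; The LoadAction event logs the file path, parses the file and, on success, sets BasePath from "path" and IsDebug from "debug" equalling "1".
; GetDataPath resolves the file name against a Data folder three levels above the project's persistent download directory.
; A failed load leaves both variables untouched.
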(event Custom|LoadAction
  ;[1 1 1] Load JSON config file
  (bind _path (CallFunction|GetDataPath (Variables|Default|GetFile)))
  (Development|PrintString (Utilities|String|Append "load config file " _path) false)
  (bind (_outjsonobject _returnvalue) (Class|JsonBlueprintFunctionLibrary|FromFile (Utilities|Struct|MakeFilePath _path)))
  (if _returnvalue
    (Utilities|FlowControl|Sequence
      (:then_0
        (bind _outvalue (|GetJsonField _outjsonobject "path"))
        (Variables|Default|SetBase%20Path _outvalue))
      (:then_1
        (bind _outvalue_2 (|GetJsonField _outjsonobject "debug"))
        (Variables|Default|SetIs%20Debug (Utilities|Enum|Equal(Enum) (Utilities|String|Append _outvalue_2 "") "1"))))))

(event EventBeginPlay)

(event EventTick
  (params (DeltaSeconds :type Float%20%28single-precision%29)))

(fn GetDataPath
  (params (file :type String))
  (return (Utilities|String|Append (Class|BlueprintPathsLibrary|ProjectPersistentDownloadDir) "../../../Data/" file)))