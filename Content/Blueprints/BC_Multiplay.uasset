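; BC_Multiplay loads and controls a group of media players together, one numbered "G" video file per player from a project-relative folder.
; Load, Play, Stop and Unload actions open, play, pause and close the players.
; Tick polls readiness and calls OnLoaded once all opened files are ready.
; End of playback is estimated from game time since Play against the last read duration, then all players rewind and OnFinish is called.
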(event Custom|StopAction
  ;[1 1 1] Play all ready files
  (for _array_element (Variables|Default|Getplayers)
    (Sequencer|Player|Pause _array_element)
    (Variables|Default|SetisPlay false)))

(event Custom|LoadAction
  (bind _isdebug (Variables|Default|GetisDebug))
  (bind _isdebug_2 (Variables|Default|GetisDebug))
  (for (_array_element _array_index) (Variables|Default|Getplayers)
    (bind _path (CallFunction|GetVideosPath (Utilities|String|Append "" "G" (Utilities|String|ToString(Integer) (+ _array_index 1)) (Variables|Default|Getextension))))
    (Development|PrintString (Utilities|String|Append (Utilities|String|ToString(Integer) _array_index) " - " (Utilities|GetDisplayName _array_element) " - " _path) _isdebug_2 _isdebug_2)
    (bind _returnvalue (Class|MediaPlayer|OpenFile _array_element _path))
    (if _returnvalue
      (Development|PrintString "open ok" _isdebug _isdebug "(R=0.000905,G=1.000000,B=0.000000,A=1.000000)")
      ;[1 1 1] Count opened files
      (bind _result (Math|Integer|IncrementInt (Variables|Default|GetcountOpened))
        (:%20%20
          (Variables|Default|SetcountOpened _result)))
      (else
        (Development|PrintString "open error!" _isdebug _isdebug "(R=1.000000,G=0.000000,B=0.061807,A=1.000000)")))))

(event Custom|UnloadAction
  ;[1 1 1] Unload
  (for _array_element (Variables|Default|Getplayers)
    (Media|MediaPlayer|Close _array_element :!class /Script/MediaAssets.MediaPlayer)
    (Variables|Default|SetisPlay false)))

(event Custom|PlayAction
  ;[1 1 1] Play all ready files
  (for _array_element (Variables|Default|Getplayers)
    (if (Class|MediaPlayer|IsReady _array_element)
      (Media|MediaPlayer|Play _array_element :!class /Script/MediaAssets.MediaPlayer)
      (Variables|Default|SetisPlay true)
      (Variables|Default|SetstartTime (Utilities|Time|GetGameTimeinSeconds)))))

(event Custom|CheckAction
  (bind _isdebug (Variables|Default|GetisDebug))
  (if (> (Variables|Default|GetcountOpened) 0)
    (if (not (Variables|Default|GetisLoaded))
      (Variables|Default|SetcountReady 0)
      (for (_array_element _array_index) (Variables|Default|Getplayers)
        (Development|PrintString (Utilities|String|Append (Utilities|String|ToString(Integer) _array_index) " - " (Utilities|String|ToString(Boolean) (Class|MediaPlayer|IsReady _array_element)) " - " (Utilities|String|ToString(Boolean) (Class|MediaPlayer|IsPreparing _array_element)) "-" (Utilities|String|ToString(Integer) (Class|MediaPlayer|GetTrackFormat _array_element "Video"))) false false "(R=0.000000,G=0.660000,B=1.000000,A=1.000000)" 0.0)
        (if (Class|MediaPlayer|IsReady _array_element)
          (Variables|Default|Setduration (Math|Timespan|GetTotalSeconds (Media|MediaPlayer|GetDuration _array_element)))
          ;[1 1 1] Count ready files increment
          (bind _result (Math|Integer|IncrementInt (Variables|Default|GetcountReady))
            (:%20%20
              (Variables|Default|SetcountReady _result)))))
      (Development|PrintString (Utilities|String|Append "counts" " - " (Utilities|String|ToString(Integer) (Variables|Default|GetcountReady)) "/" (Utilities|String|ToString(Integer) (Variables|Default|GetcountOpened))) false false)
      (if (== (Variables|Default|GetcountOpened) (Variables|Default|GetcountReady))
        (Variables|Default|SetisLoaded true)
        ;[1 1 1] Loaded all opened files
        (Default|CallOnLoaded))
      (elif (Variables|Default|GetisPlay)
        (for (_array_element_2 _array_index_2) (Variables|Default|Getplayers)
          (Development|PrintString (Utilities|String|Append (Utilities|String|ToString(Integer) _array_index_2) " - " (Utilities|String|ToString(Float) (Math|Timespan|GetTotalSeconds (Class|MediaPlayer|GetDisplayTime _array_element_2)))) (Variables|Default|GetisDebug) false "(R=0.866000,G=1.000000,B=0.059899,A=1.000000)" 0.0))
        (Development|PrintString (Utilities|String|ToString(Float) (Math|Float|Absolute(Float) (- (Variables|Default|Getduration) (- (Utilities|Time|GetGameTimeinSeconds) (Variables|Default|GetstartTime))))) (Variables|Default|GetisDebug) false "(R=1.000000,G=0.267197,B=0.336942,A=1.000000)" 0.0)
        (if (< (Math|Float|Absolute(Float) (- (Variables|Default|Getduration) (- (Utilities|Time|GetGameTimeinSeconds) (Variables|Default|GetstartTime)))) 0.2)
          (for _array_element_3 (Variables|Default|Getplayers)
            (Class|MediaPlayer|Rewind _array_element_3)
            (Variables|Default|SetisPlay false))
          (Development|PrintString "finished" _isdebug _isdebug "(R=0.866000,G=1.000000,B=0.059899,A=1.000000)" 0.0)
          (Default|CallOnFinish))))))

(event EventBeginPlay)

(event EventTick
  (params (DeltaSeconds :type Float%20%28single-precision%29))
  (CallFunction|CheckAction))

(fn GetVideosPath
  (params (file :type String))
  (return (Utilities|String|Append (Class|KismetSystemLibrary|GetProjectDirectory) (Variables|Default|GetbasePath) (Variables|Default|Getpath) "/" file)))