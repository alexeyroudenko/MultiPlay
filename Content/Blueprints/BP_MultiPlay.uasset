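; BP_MultiPlay is an actor that opens and loops several videos together through an array of media players.
; BeginPlay opens a numbered MP4 from a hard-coded local folder on each player, counting successful opens.
; Tick polls readiness until the ready count matches the opened count, then fires OnLoaded once.
; OnLoaded starts all ready players in one pass with looping enabled, so playback begins together.
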(event Custom|onLoaded
  (Development|PrintString "ready to play")
  ;[1 1 1] Play all ready files
  (for _array_element (Variables|Default|Getplayers)
    (if (Class|MediaPlayer|IsReady _array_element)
      (Components|Timeline|SetLooping _array_element true)
      (Media|MediaPlayer|Play _array_element :!class /Script/MediaAssets.MediaPlayer))))

(event EventBeginPlay
  (for (_array_element _array_index) (Variables|Default|Getplayers)
    (Development|PrintString (Utilities|String|Append (Utilities|String|ToString(Integer) _array_index) " - " (Utilities|GetDisplayName _array_element) " - " (Utilities|String|Append "C:\\Users\\W03\\Sync\\Exchange\\2023-12_MGM\\TD\\pixelmaps\\h265\\G" (Utilities|String|ToString(Integer) (+ _array_index 1)) ".mp4")))
    (bind _returnvalue (Class|MediaPlayer|OpenFile _array_element (Utilities|String|Append "C:\\Users\\W03\\Sync\\Exchange\\2023-12_MGM\\TD\\pixelmaps\\h265\\G" (Utilities|String|ToString(Integer) (+ _array_index 1)) ".mp4")))
    (if _returnvalue
      (Development|PrintString "open ok" true true "(R=0.000905,G=1.000000,B=0.000000,A=1.000000)")
      ;[1 1 1] Count opened files
      (bind _result (Math|Integer|IncrementInt (Variables|Default|GetcountOpened))
        (:%20%20
          (Variables|Default|SetcountOpened _result)))
      (else
        (Development|PrintString "open error!" true true "(R=1.000000,G=0.000000,B=0.061807,A=1.000000)")))))

(event Collision|EventActorBeginOverlap
  (params (OtherActor :type Actor%20Object%20Reference)))

(event EventTick
  (params (DeltaSeconds :type Float%20%28single-precision%29))
  (if (not (Variables|Default|GetisLoaded))
    (Variables|Default|SetcountReady 0)
    (for (_array_element _array_index) (Variables|Default|Getplayers)
      (Development|PrintString (Utilities|String|Append (Utilities|String|ToString(Integer) _array_index) " - " (Utilities|String|ToString(Boolean) (Class|MediaPlayer|IsReady _array_element)) " - ") false false "(R=0.000000,G=0.660000,B=1.000000,A=1.000000)" 0.0)
      (if (Class|MediaPlayer|IsReady _array_element)
        ;[1 1 1] Count ready files increment
        (bind _result (Math|Integer|IncrementInt (Variables|Default|GetcountReady))
          (:%20%20
            (Variables|Default|SetcountReady _result)))))
    (Development|PrintString (Utilities|String|Append "counts" " - " (Utilities|String|ToString(Integer) (Variables|Default|GetcountReady)) "/" (Utilities|String|ToString(Integer) (Variables|Default|GetcountOpened))) false false)
    (if (== (Variables|Default|GetcountOpened) (Variables|Default|GetcountReady))
      (Variables|Default|SetisLoaded true)
      (CallFunction|OnLoaded))))

(fn ConstructionScript)